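; BP_PlayerController_WTTest is a test player controller that assigns different materials to two characters.
; Its SetCharactersMaterials event casts MCharacter1 and MCharacter2 to ThirdPersonCharacter in separate sequence branches, sets each mesh's first material slot and prints a debug string.
; BeginPlay, Tick and the construction script are empty, and nothing in this Blueprint calls the event or sets the character references.
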(event `self.ReceiveBeginPlay`)

(event `self.SetCharactersMaterials`
  (`|ExecutionSequence`
    (:`then_0`
      (bind _asthird_person_character (cast `/Game/Blueprints/Characters/ThirdPersonCharacter` (`self.m_Character1`)))
      (`PrimitiveComponent.SetMaterial` (`Character.Mesh` _asthird_person_character) 0 "/Engine/VREditor/UI/ArrowMaterial.ArrowMaterial")
      (`KismetSystemLibrary.PrintString` "Hello"))
    (:`then_1`
      (bind _asthird_person_character_2 (cast `/Game/Blueprints/Characters/ThirdPersonCharacter` (`self.m_Character2`)))
      (`PrimitiveComponent.SetMaterial` (`Character.Mesh` _asthird_person_character_2) 0 "/Engine/MapTemplates/Materials/BasicAsset01.BasicAsset01")
      (`KismetSystemLibrary.PrintString` "shuirmaon"))))

(fn `UserConstructionScript`)