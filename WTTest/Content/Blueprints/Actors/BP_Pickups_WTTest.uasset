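; Pickup actor that grants a bomb, explosion range or speed upgrade to the ThirdPersonCharacter that overlaps its mesh.
; BeginPlay colors the mesh blue, red or green by pickup type.
; On overlap it raises available bombs or walk speed within limits, or sets max explosion distance to current plus one when current is within max.
; The pickup then destroys itself, even if no upgrade applies.
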(event `self.ReceiveBeginPlay`
  (bind _m_mesh (`self.m_Mesh`))
  (bind _returnvalue (`self.GetPickupType`))
  (switch `PickupTypes` _returnvalue
    (:`kAddBomb`
      (`PrimitiveComponent.SetMaterial` _m_mesh 0 "/Engine/EngineDebugMaterials/VertexColorViewMode_BlueOnly.VertexColorViewMode_BlueOnly"))
    (:`kAddExplosionExpansion`
      (`PrimitiveComponent.SetMaterial` _m_mesh 0 "/Engine/EngineDebugMaterials/VertexColorViewMode_RedOnly.VertexColorViewMode_RedOnly"))
    (:`kAddPlayerSpeed`
      (`PrimitiveComponent.SetMaterial` _m_mesh 0 "/Engine/EngineDebugMaterials/VertexColorViewMode_GreenOnly.VertexColorViewMode_GreenOnly"))))

(event `self.m_Mesh.OnComponentBeginOverlap`
  (params (OverlappedComponent :type "PrimitiveComponent Object Reference") (OtherActor :type "Actor Object Reference") (OtherComp :type "PrimitiveComponent Object Reference") (OtherBodyIndex :type Integer) (bFromSweep :type Boolean) (SweepResult :type "HitResult Structure (by ref)"))
  (bind _asthird_person_character (cast `/Game/Blueprints/Characters/ThirdPersonCharacter` OtherActor))
  (bind _returnvalue (`self.GetPickupType`))
  (switch `PickupTypes` _returnvalue
    (:`kAddBomb`
      ;[1 1 1] Add Bomb
      (if true
        (bind _returnvalue_2 (+ (`WTTestCharacter.m_NumberOfAvailableBombs` _asthird_person_character) 1))
        (if (<= _returnvalue_2 (`WTTestCharacter.m_MaxNumberOfAvailableBombs` _asthird_person_character))
          (set `WTTestCharacter.m_NumberOfAvailableBombs` _returnvalue_2 _asthird_person_character))
        ;[1 1 1] Destroy Actor
        (`self.K2_DestroyActor` :!label _label)))
    (:`kAddExplosionExpansion`
      ;[1 1 1] Add Explosion Expansion
      (if true
        (bind _m_currentexplosiontiledistance (`WTTestCharacter.m_CurrentExplosionTileDistance` _asthird_person_character))
        (if (<= _m_currentexplosiontiledistance (`WTTestCharacter.m_MaxExplosionTileDistance` _asthird_person_character))
          (set `WTTestCharacter.m_MaxExplosionTileDistance` (+ _m_currentexplosiontiledistance 1) _asthird_person_character)
          (goto _label)
          (else
            (goto _label)))))
    (:`kAddPlayerSpeed`
      ;[1 1 1] Add Speed
      (if true
        (bind _charactermovement (`Character.CharacterMovement` _asthird_person_character))
        (bind _returnvalue_3 (+ (`CharacterMovementComponent.MaxWalkSpeed` _charactermovement) 100.0))
        (if (< _returnvalue_3 1500.0)
          (set `CharacterMovementComponent.MaxWalkSpeed` _returnvalue_3 _charactermovement)
          (goto _label)
          (else
            (goto _label)))))))

(fn `UserConstructionScript`)