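; HUD for the WTTest game mode that shows in-game widgets and handles the timer-expired draw ending.
; On BeginPlay it caches the game mode and adds the game mode and players info widgets to the viewport.
; Tick polls the game mode's level timer; at zero it pauses the game, shows an animated end-game widget marked as a draw, and switches to UI-only input with the cursor visible.
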(event `self.ReceiveBeginPlay`
  (`|ExecutionSequence`
    (:`then_0`
      (bind _asbp_game_mode_wttest (cast `/Game/Blueprints/GameModes/BP_GameMode_WTTest` (`GameplayStatics.GetGameMode`)))
      (set `self.m_GameMode` _asbp_game_mode_wttest))
    (:`then_1`
      (bind _returnvalue (`|CreateWidget` "/Game/Blueprints/UserWidgets/WBP_GameModeUserWidget_WTTest.WBP_GameModeUserWidget_WTTest_C"))
      (`UserWidget.AddToViewport` _returnvalue 0))
    (:`then_2`
      (bind _returnvalue_2 (`|CreateWidget` "/Game/Blueprints/UserWidgets/WBP_PlayersInfoUserWidget_WTTest.WBP_PlayersInfoUserWidget_WTTest_C"))
      (`UserWidget.AddToViewport` _returnvalue_2 0))))

(event `self.ReceiveTick`
  (params (DeltaSeconds :type "Float (single-precision)"))
  (bind _returnvalue (`GameplayStatics.GetPlayerController` 0))
  (`|ExecutionSequence`
    (:`then_0`
      ;[1 1 1] Draw End Game
      (if (<= (`WTTestGameMode.m_LevelTimer` (`self.m_GameMode`)) 0.0)
        (`GameplayStatics.SetGamePaused` true)
        (bind _returnvalue_2 (`|CreateWidget` "/Game/Blueprints/UserWidgets/WBP_EndGameUserWidget_WTTest.WBP_EndGameUserWidget_WTTest_C" _returnvalue))
        (set `/Game/Blueprints/UserWidgets/WBP_EndGameUserWidget_WTTest.EndGameReason` "DRAW" _returnvalue_2)
        (`UserWidget.AddToViewport` _returnvalue_2 0)
        (`UserWidget.PlayAnimation` _returnvalue_2 (`/Game/Blueprints/UserWidgets/WBP_EndGameUserWidget_WTTest.Appeard` _returnvalue_2) 0.0 1 "Forward" 1.0 false)
        (`WidgetBlueprintLibrary.SetInputMode_UIOnlyEx` _returnvalue _returnvalue_2 "LockOnCapture")
        (set `PlayerController.bShowMouseCursor` true _returnvalue)))))

(fn `UserConstructionScript`)